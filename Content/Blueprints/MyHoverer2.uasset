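; MyHoverer2 is a hover vehicle Blueprint that turns the right motion controller's orientation into roll, pitch and yaw throttles every Tick.
; Offset roll and inverted pitch are clamped, normalized and shaped by a shared rotation response curve.
; Yaw compares the controller's horizontal heading with the mesh's right vector, snapping to full signed throttle when the controller does not point ahead of the mesh.
; This graph does not apply the throttles.
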(event `self.ReceiveTick`
  (params (DeltaSeconds :type "Float (single-precision)"))
  (bind _staticmeshcomponent (`self.StaticMeshComponent`))
  (bind _returnvalue (`SceneComponent.GetForwardVector` (`self.RightMotionController`)))
  (bind _returnvalue_2 (`KismetMathLibrary.DotProduct2D` (`KismetMathLibrary.MakeVector2D` (.x (`SceneComponent.GetRightVector` _staticmeshcomponent)) (.y (`SceneComponent.GetRightVector` _staticmeshcomponent))) (`KismetMathLibrary.MakeVector2D` (.x _returnvalue) (.y _returnvalue))))
  (set `self.rollThrottle` (`CurveFloat.GetFloatValue` (`self.RoitationControllerCurve`) (/ (`KismetMathLibrary.FClamp` (+ (.roll (`SceneComponent.GetSocketRotation` (`self.RightMotionController`) "None")) 45.0) -90.0 90.0) 90.0)))
  (set `self.pitchThrottle` (`CurveFloat.GetFloatValue` (`self.RoitationControllerCurve`) (/ (`KismetMathLibrary.FClamp` (* (.pitch (`SceneComponent.GetSocketRotation` (`self.RightMotionController`) "None")) -1.0) -45.0 45.0) 45.0)))
  (if (> (`KismetMathLibrary.DotProduct2D` (`KismetMathLibrary.MakeVector2D` (.x (`SceneComponent.GetForwardVector` _staticmeshcomponent)) (.y (`SceneComponent.GetForwardVector` _staticmeshcomponent))) (`KismetMathLibrary.MakeVector2D` (.x _returnvalue) (.y _returnvalue))) 0.0)
    (set `self.yawThrottle` _returnvalue_2)
    (else
      (set `self.yawThrottle` (* (`KismetMathLibrary.SignOfFloat` _returnvalue_2) 1.0)))))

(fn `UserConstructionScript`)